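; BP_LinkProxy is a smart nav link proxy that makes AI-driven characters jump when they reach the link.
; On SmartLinkReached it casts the agent to BaseCharacter and checks the sign of its Y velocity, with the Left flag selecting which direction counts as a match.
; A matching agent jumps immediately, while any other jumps after a short delay.
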(event `self.ReceiveBeginPlay`)

(event `self.ReceiveSmartLinkReached`
  (params (Agent :type "Actor Object Reference") (Destination :type "Vector Structure (by ref)"))
  (bind _asbase_character (cast `BaseCharacter` Agent))
  (bind (_velocity_x _velocity_y) (`KismetMathLibrary.BreakVector` (`MovementComponent.Velocity` (`Character.CharacterMovement` _asbase_character))))
  (if (select `bool` (`self.Left`) :`false` (<= _velocity_y 0.0) :`true` (>= _velocity_y 0.0))
    (`Character.Jump` _asbase_character)
    (else
      (`KismetSystemLibrary.Delay` 0.2)
      (`Character.Jump` _asbase_character))))

(fn `UserConstructionScript`)