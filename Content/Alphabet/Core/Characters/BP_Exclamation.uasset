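; BP_Exclamation is the Exclamation character in the Alphabet game, set up here for AI control.
; On BeginPlay it assigns BT_Comma, a behavior tree named for Comma rather than Exclamation, to its BP_AiController, and does nothing if that cast fails.
; InitHealthWidgetBlueprint creates a WBP_HealthBar for its health widget only when the PlayerState marks it as a bot.
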(event `self.ReceiveBeginPlay`
  (bind _asbp_ai_controller (cast `/Game/Alphabet/Core/AI/BP_AiController` (`AIBlueprintHelperLibrary.GetAIController` self)))
  (set `/Game/Alphabet/Core/AI/BP_AiController.BehaviorTree` "/Game/Alphabet/Core/AI/BehaviorTrees/BT_Comma.BT_Comma" _asbp_ai_controller))

(event `self.InitHealthWidgetBlueprint`
  (if (`PlayerState.bIsABot` (`self.PlayerState`))
    (bind _returnvalue (`|CreateWidget` "/Game/Alphabet/Core/UI/WBP_HealthBar.WBP_HealthBar_C" null self))
    (`WidgetComponent.SetWidget` (`self.HealthWidget`) _returnvalue)))

(fn `UserConstructionScript`)