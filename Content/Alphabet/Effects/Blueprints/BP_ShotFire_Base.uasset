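; BP_ShotFire_Base is a base fire-shot effect actor that explodes when its Sphere collision overlaps any actor other than its owner.
; On overlap it spawns the HitParticle emitter at the FX component's location and applies full, non-falloff radial damage around itself.
; The damage ignores and credits the owner, passes the instigator controller and uses Pawn as the prevention channel, then the actor destroys itself.
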(event `self.Sphere.OnComponentBeginOverlap`
  (params (OverlappedComponent :type "PrimitiveComponent Object Reference") (OtherActor :type "Actor Object Reference") (OtherComp :type "PrimitiveComponent Object Reference") (OtherBodyIndex :type Integer) (bFromSweep :type Boolean) (SweepResult :type "HitResult Structure (by ref)"))
  (if (!= OtherActor (`self.GetOwner`))
    (`GameplayStatics.SpawnEmitterAtLocation` (`self.HitParticle`) (`SceneComponent.K2_GetComponentLocation` (`self.FX`)) (`KismetMathLibrary.Conv_VectorToRotator` (`KismetMathLibrary.Vector_Zero`)) (`KismetMathLibrary.Vector_One`))
    (`GameplayStatics.ApplyRadialDamage` 100.0 (`self.K2_GetActorLocation`) 200.0 null (`|MakeArray` (`self.GetOwner`)) (`self.GetOwner`) (`self.GetInstigatorController`) true (enumliteral `ECollisionChannel` "ECC_Pawn"))
    (`self.K2_DestroyActor`)))

(fn `UserConstructionScript`)